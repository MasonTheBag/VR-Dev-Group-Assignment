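; Pressable button that visually depresses when a VR pawn overlaps its collision component.
; BeginPlay caches the relative location of ButtonTop as the rest position.
; Overlap begin moves the top down along local Z with a short MoveComponentTo, and overlap end returns it to rest after a brief delay.
; The Blueprint only animates the button and triggers no other logic.
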(event OnComponentBeginOverlap(Collision)
  (params (OverlappedComponent :type Primitive%20Component%20Object%20Reference) (OtherActor :type Actor%20Object%20Reference) (OtherComp :type Primitive%20Component%20Object%20Reference) (OtherBodyIndex :type Integer) (bFromSweep :type Boolean) (SweepResult :type Hit%20Result%20Structure%20%28by%20ref%29))
  (Utilities|Casting|CastToVRPawn OtherActor)
  (Components|MoveComponentTo (Variables|Default|GetButtonTop) (- (Variables|Default|GetstartLocation) "0.000000,0.000000,10.000000") "0, 0, 0" false false 0.1 false))

(event OnComponentEndOverlap(Collision)
  (params (OverlappedComponent :type Primitive%20Component%20Object%20Reference) (OtherActor :type Actor%20Object%20Reference) (OtherComp :type Primitive%20Component%20Object%20Reference) (OtherBodyIndex :type Integer))
  (Utilities|Casting|CastToVRPawn OtherActor)
  (Utilities|FlowControl|Delay 0.1)
  (Components|MoveComponentTo (Variables|Default|GetButtonTop) (Variables|Default|GetstartLocation) "0, 0, 0" false false 0.1 false))

(event EventBeginPlay
  (Variables|Default|SetstartLocation (Variables|/Script/Engine.SceneComponent|GetRelativeLocation (Variables|Default|GetButtonTop))))

(fn ConstructionScript)